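; BP_Finish is the finish-line actor that ends a timed run when the Player overlaps it.
; It flags the player as finished, calls their total time calculation, then copies current and total times from ThirdPersonGameMode into the Player_GI game instance.
; It overwrites the personal best only when minutes are not higher and seconds are lower.
; It also stops the music, clears the first-run flag and opens the Scoreboard level.
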(event Collision|EventActorBeginOverlap
  (params (OtherActor :type Actor%20Object%20Reference))
  (bind _returnvalue (Game|GetGameInstance))
  (bind _asplayer_gi (Utilities|Casting|CastToPlayer_GI _returnvalue))
  (bind _asplayer (Utilities|Casting|CastToPlayer OtherActor))
  (Variables|/Game/Blueprints/Player/Player.Player_C|SetFinish _asplayer true)
  (Default|CalculateTotalTime _asplayer)
  (bind _asthird_person_game_mode (Utilities|Casting|CastToThirdPersonGameMode (Game|GetGameMode)))
  (Variables|/Game/Blueprints/Player/Player_GI.Player_GI_C|SetNbSecondesCurrentRun _asplayer_gi (Variables|/Game/Blueprints/Player/ThirdPersonGameMode.ThirdPersonGameMode_C|GetSecondes_CurrentRun _asthird_person_game_mode))
  (Variables|/Game/Blueprints/Player/Player_GI.Player_GI_C|SetNbMinutesCurrentRun _asplayer_gi (Variables|/Game/Blueprints/Player/ThirdPersonGameMode.ThirdPersonGameMode_C|GetMinutes_CurrentRun _asthird_person_game_mode))
  (Variables|/Game/Blueprints/Player/Player_GI.Player_GI_C|SetNbSecondesTotales _asplayer_gi (Variables|/Game/Blueprints/Player/ThirdPersonGameMode.ThirdPersonGameMode_C|GetTotalesSecondes _asthird_person_game_mode))
  (Variables|/Game/Blueprints/Player/Player_GI.Player_GI_C|SetNbMinutesTotales _asplayer_gi (Variables|/Game/Blueprints/Player/ThirdPersonGameMode.ThirdPersonGameMode_C|GetTotalesMinutes _asthird_person_game_mode))
  (Default|StopMusique _asthird_person_game_mode)
  (if (<= (Variables|/Game/Blueprints/Player/ThirdPersonGameMode.ThirdPersonGameMode_C|GetMinutes_CurrentRun _asthird_person_game_mode) (Variables|/Game/Blueprints/Player/Player_GI.Player_GI_C|GetNbMinutesPB _asplayer_gi))
    (if (< (Variables|/Game/Blueprints/Player/ThirdPersonGameMode.ThirdPersonGameMode_C|GetSecondes_CurrentRun _asthird_person_game_mode) (Variables|/Game/Blueprints/Player/Player_GI.Player_GI_C|GetNbSecondesPB _asplayer_gi))
      (Variables|/Game/Blueprints/Player/Player_GI.Player_GI_C|SetNbMinutesPB _asplayer_gi (Variables|/Game/Blueprints/Player/ThirdPersonGameMode.ThirdPersonGameMode_C|GetMinutes_CurrentRun _asthird_person_game_mode))
      (Variables|/Game/Blueprints/Player/Player_GI.Player_GI_C|SetNbSecondesPB _asplayer_gi (Variables|/Game/Blueprints/Player/ThirdPersonGameMode.ThirdPersonGameMode_C|GetSecondes_CurrentRun _asthird_person_game_mode))))
  (if (Variables|/Game/Blueprints/Player/Player_GI.Player_GI_C|GetFirstRun _asplayer_gi)
    (Variables|/Game/Blueprints/Player/Player_GI.Player_GI_C|SetFirstRun _asplayer_gi false)
    (Development|PrintString "Hello"))
  (Game|OpenLevel(byName) "Scoreboard"))

(fn ConstructionScript)