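; BP_Spick is a spike trap that raises pikes to a configurable height and kills the player on contact.
; The Spick timeline drives the pikes' Z position, with an event track flip-flopping SpickActive to mark the lethal window.
; It either loops endlessly through an array of delays or fires when the player enters Box, then resets.
; Tick polls overlaps to retrigger the trap and to apply death, sound and ragdoll.
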(event OnComponentBeginOverlap(Box)
  (params (OverlappedComponent :type Primitive%20Component%20Object%20Reference) (OtherActor :type Actor%20Object%20Reference) (OtherComp :type Primitive%20Component%20Object%20Reference) (OtherBodyIndex :type Integer) (bFromSweep :type Boolean) (SweepResult :type Hit%20Result%20Structure%20%28by%20ref%29))
  (bind _sm_pikes_part03 (Variables|Default|GetSM_Pikes_part03))
  (bind _relativelocation (Variables|/Script/Engine.SceneComponent|GetRelativeLocation _sm_pikes_part03))
  (Utilities|Casting|CastToPlayer OtherActor)
  (bind _movement (Timeline|Spick PlayFromStart)
    (:Update
      ;[1 1 1] Déplacement des piques
      (Transformation|SetRelativeLocation _sm_pikes_part03 (Math|Vector|MakeVector (.x _relativelocation) (.y _relativelocation) (Math|Float|MapRangeClamped _movement 0.0 1.0 -4e+01 (Variables|Default|GetHeight))) false false))
    (:Finished
      (if (Variables|Default|GetIsInfinite)
        ;[1 1 1] Delay
        (Utilities|FlowControl|Delay (Utilities|Array|Get(acopy) (Variables|Default|GetDelay) (Variables|Default|GetCount)))
        (Variables|Default|SetCount (Math|Integer|SelectInt 0 (+ (Variables|Default|GetCount) 1) (> (+ (Variables|Default|GetCount) 1) (Utilities|Array|LastIndex (Variables|Default|GetDelay)))))
        (CallFunction|SpickLoop)
        ;[0.1419 0.5265 1] Position Son
        (Audio|PlaySoundatLocation "/Game/Sound/TRAP/CUE_TRAP_Pick.CUE_TRAP_Pick" (Transformation|GetActorLocation (Components|GetOwner (Variables|Default|GetSM_Pikes_part03))) "0, 0, 0" 1.0 1.0 0.0 0 0 0)
        (else
          (CallFunction|ResetTimeline)
          (Utilities|FlowControl|Delay 0.5)
          (CallFunction|ResetDoOnce))))
    (:SetBool
      ;[1 1 1] CanNIQUERLAMEREDUPLAYER
      (bind _isa (Utilities|FlowControl|FlipFlop)
        (:A
          _)
        (:B
          _))
      (Variables|Default|SetSpickActive _isa))))

(event Custom|ResetTimeline
  (bind _sm_pikes_part03 (Variables|Default|GetSM_Pikes_part03))
  (bind _relativelocation (Variables|/Script/Engine.SceneComponent|GetRelativeLocation _sm_pikes_part03))
  (bind _movement (Timeline|Spick SetNewTime)
    (:Update
      ;[1 1 1] Déplacement des piques
      (Transformation|SetRelativeLocation _sm_pikes_part03 (Math|Vector|MakeVector (.x _relativelocation) (.y _relativelocation) (Math|Float|MapRangeClamped _movement 0.0 1.0 -4e+01 (Variables|Default|GetHeight))) false false))
    (:Finished
      (if (Variables|Default|GetIsInfinite)
        ;[1 1 1] Delay
        (Utilities|FlowControl|Delay (Utilities|Array|Get(acopy) (Variables|Default|GetDelay) (Variables|Default|GetCount)))
        (Variables|Default|SetCount (Math|Integer|SelectInt 0 (+ (Variables|Default|GetCount) 1) (> (+ (Variables|Default|GetCount) 1) (Utilities|Array|LastIndex (Variables|Default|GetDelay)))))
        (CallFunction|SpickLoop)
        ;[0.1419 0.5265 1] Position Son
        (Audio|PlaySoundatLocation "/Game/Sound/TRAP/CUE_TRAP_Pick.CUE_TRAP_Pick" (Transformation|GetActorLocation (Components|GetOwner (Variables|Default|GetSM_Pikes_part03))) "0, 0, 0" 1.0 1.0 0.0 0 0 0)
        (else
          (CallFunction|ResetTimeline)
          (Utilities|FlowControl|Delay 0.5)
          (CallFunction|ResetDoOnce))))
    (:SetBool
      ;[1 1 1] CanNIQUERLAMEREDUPLAYER
      (bind _isa (Utilities|FlowControl|FlipFlop)
        (:A
          _)
        (:B
          _))
      (Variables|Default|SetSpickActive _isa))))

(event Custom|SpickLoop
  (bind _sm_pikes_part03 (Variables|Default|GetSM_Pikes_part03))
  (bind _relativelocation (Variables|/Script/Engine.SceneComponent|GetRelativeLocation _sm_pikes_part03))
  (bind _movement (Timeline|Spick PlayFromStart)
    (:Update
      ;[1 1 1] Déplacement des piques
      (Transformation|SetRelativeLocation _sm_pikes_part03 (Math|Vector|MakeVector (.x _relativelocation) (.y _relativelocation) (Math|Float|MapRangeClamped _movement 0.0 1.0 -4e+01 (Variables|Default|GetHeight))) false false))
    (:Finished
      (if (Variables|Default|GetIsInfinite)
        ;[1 1 1] Delay
        (Utilities|FlowControl|Delay (Utilities|Array|Get(acopy) (Variables|Default|GetDelay) (Variables|Default|GetCount)))
        (Variables|Default|SetCount (Math|Integer|SelectInt 0 (+ (Variables|Default|GetCount) 1) (> (+ (Variables|Default|GetCount) 1) (Utilities|Array|LastIndex (Variables|Default|GetDelay)))))
        (CallFunction|SpickLoop)
        ;[0.1419 0.5265 1] Position Son
        (Audio|PlaySoundatLocation "/Game/Sound/TRAP/CUE_TRAP_Pick.CUE_TRAP_Pick" (Transformation|GetActorLocation (Components|GetOwner (Variables|Default|GetSM_Pikes_part03))) "0, 0, 0" 1.0 1.0 0.0 0 0 0)
        (else
          (CallFunction|ResetTimeline)
          (Utilities|FlowControl|Delay 0.5)
          (CallFunction|ResetDoOnce))))
    (:SetBool
      ;[1 1 1] CanNIQUERLAMEREDUPLAYER
      (bind _isa (Utilities|FlowControl|FlipFlop)
        (:A
          _)
        (:B
          _))
      (Variables|Default|SetSpickActive _isa))))

(event Custom|ResetDoOnce
  (Utilities|FlowControl|DoOnce false) ; enters at Reset
)

(event EventTick
  (params (DeltaSeconds :type Float%20%28single-precision%29))
  (bind _returnvalue (Game|GetPlayerCharacter 0))
  (bind _returnvalue_2 (Game|GetPlayerCharacter 0))
  (bind _asplayer (Utilities|Casting|CastToPlayer _returnvalue))
  (bind _asplayer_2 (Utilities|Casting|CastToPlayer _returnvalue_2))
  (Utilities|FlowControl|Sequence
    (:then_0
      ;[1 1 1] Detecte si le player prend des dégats
      (if (Variables|Default|GetSpickActive)
        (if (Collision|IsOverlappingActor (Variables|Default|GetSM_Pikes_part03) _asplayer_2 :!class /Script/Engine.PrimitiveComponent)
          (Utilities|FlowControl|DoOnce false
            (:Completed
              (Audio|PlaySound2D "/Game/Sound/CHARA/CUE_CHA_Slashed.CUE_CHA_Slashed" 1.0 1.0 0.0 0 0)
              (Variables|/Game/Blueprints/Player/Player.Player_C|SetIsDead _asplayer_2 true)
              (Default|Ragdoll _asplayer_2))))))
    (:then_1
      (if (Collision|IsOverlappingActor (Variables|Default|GetBox) _asplayer :!class /Script/Engine.PrimitiveComponent)
        (Utilities|FlowControl|DoOnce false
          (:Completed
            (if (not (Variables|/Game/Blueprints/Player/Player.Player_C|GetIsDead _asplayer))
              (CallFunction|SpickLoop))))))))

(event EventBeginPlay
  (Components|Timeline|SetPlayRate (Variables|Default|GetSpick) (Variables|Default|GetPlayRate))
  (if (Variables|Default|GetIsInfinite)
    (CallFunction|SpickLoop)))

(fn ConstructionScript)