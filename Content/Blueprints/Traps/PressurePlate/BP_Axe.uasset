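; Swinging pendulum axe trap that kills the player on contact.
; On BeginPlay, the Pendule timeline starts at a configurable play rate and drives Scene1's pitch, playing a whoosh sound as the swing nears vertical.
; A player overlapping the Box triggers, only once, a slash sound, death flag, ragdoll and capsule impulse scaled from the trap actor's GetVelocity.
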(event OnComponentBeginOverlap(Box)
  (params (OverlappedComponent :type Primitive%20Component%20Object%20Reference) (OtherActor :type Actor%20Object%20Reference) (OtherComp :type Primitive%20Component%20Object%20Reference) (OtherBodyIndex :type Integer) (bFromSweep :type Boolean) (SweepResult :type Hit%20Result%20Structure%20%28by%20ref%29))
  ;[1 1 1] Transforme le joueur en saucisson
  (bind _asplayer (Utilities|Casting|CastToPlayer OtherActor))
  (Utilities|FlowControl|DoOnce false
    (:Completed
      (Audio|PlaySound2D "/Game/Sound/CHARA/CUE_CHA_Slashed.CUE_CHA_Slashed" 1.0 1.0 0.0 0 0)
      (Variables|/Game/Blueprints/Player/Player.Player_C|SetIsDead _asplayer true)
      (Default|Ragdoll _asplayer)
      (Physics|AddImpulse (Variables|/Script/Engine.Character|GetCapsuleComponent _asplayer) (* (Transformation|GetVelocity) 10) "None" true))))

(event Custom|PenduleAxe
  ;[1 1 1] Loop - Pendule
  (bind _rotate (Timeline|Pendule PlayFromStart)
    (:Update
      (Transformation|SetRelativeRotation (Variables|Default|GetScene1) (Math|Rotator|MakeRotator 0.0 _rotate 0.0) false false)
      ;[0 0.4125 1] Son mouvement Axe
      (if (Math|Float|InRange(Float) _rotate -5.0 5.0)
        (Audio|PlaySoundatLocation "/Game/Sound/TRAP/CUE_TRAP_Axe.CUE_TRAP_Axe" (Transformation|GetActorLocation (Components|GetOwner (Variables|Default|GetPiegeHache02ForUE))) "0, 0, 0" 1.0 1.0 0.0 0 0 0)))))

(event EventBeginPlay
  ;[1 1 1] Begin play
  (Components|Timeline|SetPlayRate (Variables|Default|GetPendule) (Variables|Default|GetPlayRate))
  (CallFunction|PenduleAxe))

(fn ConstructionScript)