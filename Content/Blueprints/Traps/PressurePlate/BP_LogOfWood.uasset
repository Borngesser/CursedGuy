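; Swinging log trap that knocks the player away, triggered once per cycle when the Player enters the Boxtavu detection box.
; The Smash timeline rolls the Arrow component down and raises CanSmash through an event track.
; While that flag is set, Tick launches any Player overlapping the Sphere along Cylinder1's forward vector with upward lift.
; After the swing, a delay and Reload timeline restore the log and re-arm the trigger.
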(event OnComponentBeginOverlap(Boxtavu)
  (params (OverlappedComponent :type Primitive%20Component%20Object%20Reference) (OtherActor :type Actor%20Object%20Reference) (OtherComp :type Primitive%20Component%20Object%20Reference) (OtherBodyIndex :type Integer) (bFromSweep :type Boolean) (SweepResult :type Hit%20Result%20Structure%20%28by%20ref%29))
  ;[1 1 1] Le marteau tape ?
  (Utilities|Casting|CastToPlayer OtherActor)
  (Utilities|FlowControl|DoOnce false
    (:Completed
      (CallFunction|Hammer))))

(event Custom|Hammer
  (bind _arrow (Variables|Default|GetArrow))
  (bind _arrow_2 (Variables|Default|GetArrow))
  (bind _relativerotation (Variables|/Script/Engine.SceneComponent|GetRelativeRotation _arrow_2))
  (bind _relativerotation_2 (Variables|/Script/Engine.SceneComponent|GetRelativeRotation _arrow))
  ;[1 1 1] Smash du marteau
  (Audio|PlaySoundatLocation "/Game/Sound/TRAP/CUE_TRAP_Wood.CUE_TRAP_Wood" (Transformation|GetActorLocation (Components|GetOwner (Variables|Default|GetArrow))) "0, 0, 0" 1.0 1.0 0.0 0 0 0)
  (bind _newtrack_0 (Timeline|Smash PlayFromStart)
    (:Update
      (Transformation|SetRelativeRotation _arrow (Math|Rotator|MakeRotator (Math|Float|MapRangeClamped _newtrack_0 0.0 1.0 0.0 -9e+01) (.pitch _relativerotation_2) (.yaw _relativerotation_2)) false false))
    (:Finished
      ;[1 1 1] Se place au milieu
      (Variables|Default|SetcanSmash false)
      (Utilities|FlowControl|Delay 4.0)
      (bind _newtrack_0_2 (Timeline|Reload PlayFromStart)
        (:Update
          (Transformation|SetRelativeRotation _arrow_2 (Math|Rotator|MakeRotator (Math|Float|MapRangeClamped _newtrack_0_2 0.0 1.0 -9e+01 0.0) (.pitch _relativerotation) (.yaw _relativerotation)) false false))
        (:Finished
          ;[1 1 1] Le marteau tape ?
          (Utilities|FlowControl|DoOnce false) ; enters at Reset
        )))
    (:SetBool
      (Variables|Default|SetcanSmash true))))

(event EventBeginPlay
  ;[1 1 1] Begin play
  (Components|Timeline|SetPlayRate (Variables|Default|GetSmash) (Variables|Default|GetPlayRate)))

(event EventTick
  (params (DeltaSeconds :type Float%20%28single-precision%29))
  (bind _returnvalue (Game|GetPlayerCharacter 0))
  (bind _cylinder1 (Variables|Default|GetCylinder1))
  (bind _power (Variables|Default|GetPower))
  (bind _returnvalue_2 (Math|Vector|GetForwardVector _cylinder1))
  (bind _asplayer (Utilities|Casting|CastToPlayer _returnvalue))
  (bind _returnvalue_3 (* _returnvalue_2 _power))
  ;[1 1 1] Le joueur prend des dégats ou pas ?
  (if (Variables|Default|GetcanSmash)
    (if (Collision|IsOverlappingActor (Variables|Default|GetSphere) _asplayer :!class /Script/Engine.PrimitiveComponent)
      (Character|LaunchCharacter _asplayer (Math|Vector|MakeVector (.x _returnvalue_3) (.y _returnvalue_3) 5e+02) true true)
      (Audio|PlaySound2D "/Game/Sound/CHARA/CUE_CHA_Hit.CUE_CHA_Hit" 1.0 1.0 0.0 0 0))))

(fn ConstructionScript)