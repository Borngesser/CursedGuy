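; Bear trap Blueprint that kills a Player on overlap, snapping them to the trap's center and playing a trap sound.
; It sets IsDead, disables movement, rotation and jumping through CanMove, and ragdolls the mesh.
; Two timelines, started in the same sequence without delay, both drive the world roll of the two jaw components.
; CanMove applies speed and rotation to its target, but sets CanJump on player character 0.
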(event Collision|EventActorBeginOverlap
  (params (OtherActor :type Actor%20Object%20Reference))
  (bind _returnvalue (Transformation|GetActorLocation))
  (bind _asplayer (Utilities|Casting|CastToPlayer OtherActor))
  (Components|Movement|StopMovementImmediately (Variables|/Script/Engine.Character|GetCharacterMovement _asplayer))
  (Transformation|SetActorLocation _asplayer (Math|Vector|MakeVector (.x _returnvalue) (.y _returnvalue) (.z (Transformation|GetActorLocation _asplayer))) true false)
  (Audio|PlaySoundatLocation "/Game/Sound/TRAP/TRAP_BearTrap.TRAP_BearTrap" (Transformation|GetActorLocation) "0, 0, 0" 1.0 1.0 0.0 0 0 0)
  (Utilities|FlowControl|Sequence
    (:then_0
      (bind (_direction __50 _50) (Timeline|Timeline_0 PlayFromStart)
        (:Update
          (Transformation|SetWorldRotation (Variables|Default|GetPiegeOursForUE_PiegeOurs) (Math|Rotator|MakeRotator __50 0.0 0.0) false false)
          (Transformation|SetWorldRotation (Variables|Default|GetPiegeOursForUE_PiegeOurs1) (Math|Rotator|MakeRotator _50 0.0 0.0) false false))))
    (:then_1
      (Variables|/Game/Blueprints/Player/Player.Player_C|SetIsDead _asplayer true)
      (CallFunction|CanMove false false false _asplayer)
      (Physics|SetSimulatePhysics (Variables|/Script/Engine.Character|GetMesh _asplayer) true)
      (Collision|SetCollisionProfileName (Variables|/Script/Engine.Character|GetMesh _asplayer) "Ragdoll" true :!class /Script/Engine.PrimitiveComponent)
      (bind (_direction_2 __50_2 _50_2) (Timeline|Timeline_1 PlayFromStart)
        (:Update
          (Transformation|SetWorldRotation (Variables|Default|GetPiegeOursForUE_PiegeOurs) (Math|Rotator|MakeRotator __50_2 0.0 0.0) false false)
          (Transformation|SetWorldRotation (Variables|Default|GetPiegeOursForUE_PiegeOurs1) (Math|Rotator|MakeRotator _50_2 0.0 0.0) false false))))))

(fn ConstructionScript)

(fn CanMove
  (params (Can%20Move :type Boolean) (CanRotate :type Boolean) (CanJump :type Boolean) (Target :type Character%20Object%20Reference))
  (bind _returnvalue (Game|GetPlayerCharacter 0))
  (bind _charactermovement (Variables|/Script/Engine.Character|GetCharacterMovement Target))
  (bind _asplayer (Utilities|Casting|CastToPlayer _returnvalue))
  (if Can%20Move
    (Variables|/Script/Engine.CharacterMovementComponent|SetMaxWalkSpeed _charactermovement 6e+02)
    (else
      (Variables|/Script/Engine.CharacterMovementComponent|SetMaxWalkSpeed _charactermovement 0.0)))
  (if CanRotate
    (Variables|/Script/Engine.CharacterMovementComponent|SetRotationRate _charactermovement "0,540.000000, 0")
    (else
      (Variables|/Script/Engine.CharacterMovementComponent|SetRotationRate _charactermovement "0, 0, 0")))
  (if CanJump
    (Variables|/Game/Blueprints/Player/Player.Player_C|SetCanJump? _asplayer true)
    (else
      (Variables|/Game/Blueprints/Player/Player.Player_C|SetCanJump? _asplayer false))))