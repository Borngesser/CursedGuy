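; BP_Arrow is an arrow trap that fires projectiles continuously from the moment play begins.
; A self-calling Arrow event spawns a scaled BP_Arrow_Projectile at the Scene component's world location and rotation, then waits.
; Each wait comes from the Delay array, with Count wrapping to zero past the last index to form a repeating rhythm.
; The construction script applies the Mesh variable to the static mesh.
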(event Custom|Arrow
  (bind _scene (Variables|Default|GetScene))
  (bind _returnvalue (Transformation|GetWorldRotation _scene))
  ;[1 1 1] Spawn du projectile
  (Game|SpawnActorfromClass "/Game/Blueprints/Traps/PressurePlate/BP_Arrow_Projectile.BP_Arrow_Projectile_C" (Math|Transform|MakeTransform (Transformation|GetWorldLocation _scene) (Math|Rotator|MakeRotator (.roll _returnvalue) (.pitch _returnvalue) (.yaw _returnvalue)) "0.200000,0.200000,0.500000") "Undefined" 0 0)
  (Utilities|FlowControl|Delay (Utilities|Array|Get(acopy) (Variables|Default|GetDelay) (Variables|Default|GetCount)))
  (Variables|Default|SetCount (Math|Integer|SelectInt 0 (+ (Variables|Default|GetCount) 1) (> (+ (Variables|Default|GetCount) 1) (Utilities|Array|LastIndex (Variables|Default|GetDelay)))))
  (CallFunction|Arrow))

(event EventBeginPlay
  ;[1 1 1] Begin play
  (CallFunction|Arrow))

(fn ConstructionScript
  (Components|StaticMesh|SetStaticMesh (Variables|Default|GetStaticMesh) (Variables|Default|GetMesh)))