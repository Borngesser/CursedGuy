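; Moving trap that repeatedly thrusts a mesh outward and knocks the player away.
; The Avance timeline extends the mesh along local X, Retour drives its return, then a delay cycled from an array precedes the next push.
; Tick launches the player along the mesh's forward vector with an upward boost when overlapping the Box, except during return and delay.
; The construction script applies the configurable mesh.
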(event Custom|EventPush
  (Variables|Default|SetReloading? false)
  (bind _newtrack_0 (Timeline|Avance PlayFromStart)
    (:Update
      ;[1 1 1] Fonce
      (Transformation|SetRelativeLocation (Variables|Default|GetStaticMesh) (Math|Vector|Lerp(Vector) "0, 0, 0" (Variables|Default|GetFinishLocation) _newtrack_0) false false))
    (:Finished
      (Variables|Default|SetReloading? true)
      ;[1 1 1] Reviens à sa place
      (bind _retour (Timeline|Retour PlayFromStart)
        (:Update
          (Transformation|SetRelativeLocation (Variables|Default|GetStaticMesh) (Math|Vector|Lerp(Vector) "0, 0, 0" (Variables|Default|GetFinishLocation) _retour) false false))
        (:Finished
          ;[1 1 1] Delay
          (Utilities|FlowControl|Delay (Utilities|Array|Get(acopy) (Variables|Default|GetDelay) (Variables|Default|GetCount)))
          (Variables|Default|SetCount (Math|Integer|SelectInt 0 (+ (Variables|Default|GetCount) 1) (> (+ (Variables|Default|GetCount) 1) (Utilities|Array|LastIndex (Variables|Default|GetDelay)))))
          (CallFunction|EventPush))))))

(event EventBeginPlay
  ;[1 1 1] Begin play
  (Variables|Default|SetFinishLocation (* "1.000000, 0, 0" (Variables|Default|GetDist)))
  (Components|Timeline|SetPlayRate (Variables|Default|GetAvance) (Variables|Default|GetPlayRate))
  (CallFunction|EventPush))

(event EventTick
  (params (DeltaSeconds :type Float%20%28single-precision%29))
  (bind _returnvalue (Game|GetPlayerCharacter 0))
  (bind _staticmesh (Variables|Default|GetStaticMesh))
  (bind _power (Variables|Default|GetPower))
  (bind _returnvalue_2 (Math|Vector|GetForwardVector _staticmesh))
  (bind _asthird_person_character (Utilities|Casting|CastToThirdPersonCharacter _returnvalue))
  (bind _returnvalue_3 (* _returnvalue_2 _power))
  ;[1 1 1] Propulse le joueur si il touche la box
  (if (not (Variables|Default|GetReloading?))
    (if (Collision|IsOverlappingActor (Variables|Default|GetBox) _asthird_person_character :!class /Script/Engine.PrimitiveComponent)
      (Character|LaunchCharacter _asthird_person_character (Math|Vector|MakeVector (.x _returnvalue_3) (.y _returnvalue_3) 5e+02) true true))))

(fn ConstructionScript
  (Components|StaticMesh|SetStaticMesh (Variables|Default|GetStaticMesh) (Variables|Default|GetMesh)))