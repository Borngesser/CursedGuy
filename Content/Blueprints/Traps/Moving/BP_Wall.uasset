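; Moving crusher trap: two wall meshes slide toward each other along X and destroy the player character when both side boxes overlap it.
; Two timelines lerp the walls inward and back, looping with pauses cycled from a Delay array.
; Box overlaps set the flags checked on Tick and zero the character's ground friction until exit.
; The construction script applies configurable meshes and spaces them by Distance.
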(event OnComponentBeginOverlap(BoxDroite)
  (params (OverlappedComponent :type Primitive%20Component%20Object%20Reference) (OtherActor :type Actor%20Object%20Reference) (OtherComp :type Primitive%20Component%20Object%20Reference) (OtherBodyIndex :type Integer) (bFromSweep :type Boolean) (SweepResult :type Hit%20Result%20Structure%20%28by%20ref%29))
  (bind _asthird_person_character (Utilities|Casting|CastToThirdPersonCharacter OtherActor))
  (Variables|Default|SetOverlapDroite true)
  (Variables|/Script/Engine.CharacterMovementComponent|SetGroundFriction (Variables|/Script/Engine.Character|GetCharacterMovement _asthird_person_character) 0.0))

(event OnComponentBeginOverlap(BoxGauche)
  (params (OverlappedComponent :type Primitive%20Component%20Object%20Reference) (OtherActor :type Actor%20Object%20Reference) (OtherComp :type Primitive%20Component%20Object%20Reference) (OtherBodyIndex :type Integer) (bFromSweep :type Boolean) (SweepResult :type Hit%20Result%20Structure%20%28by%20ref%29))
  (bind _asthird_person_character (Utilities|Casting|CastToThirdPersonCharacter OtherActor))
  (Variables|Default|SetOverlapGauche true)
  (Variables|/Script/Engine.CharacterMovementComponent|SetGroundFriction (Variables|/Script/Engine.Character|GetCharacterMovement _asthird_person_character) 0.0))

(event OnComponentEndOverlap(BoxDroite)
  (params (OverlappedComponent :type Primitive%20Component%20Object%20Reference) (OtherActor :type Actor%20Object%20Reference) (OtherComp :type Primitive%20Component%20Object%20Reference) (OtherBodyIndex :type Integer))
  (bind _asthird_person_character (Utilities|Casting|CastToThirdPersonCharacter OtherActor))
  (Variables|Default|SetOverlapDroite false)
  (Variables|/Script/Engine.CharacterMovementComponent|SetGroundFriction (Variables|/Script/Engine.Character|GetCharacterMovement _asthird_person_character) 8.0))

(event OnComponentEndOverlap(BoxGauche)
  (params (OverlappedComponent :type Primitive%20Component%20Object%20Reference) (OtherActor :type Actor%20Object%20Reference) (OtherComp :type Primitive%20Component%20Object%20Reference) (OtherBodyIndex :type Integer))
  (bind _asthird_person_character (Utilities|Casting|CastToThirdPersonCharacter OtherActor))
  (Variables|Default|SetOverlapGauche false)
  (Variables|/Script/Engine.CharacterMovementComponent|SetGroundFriction (Variables|/Script/Engine.Character|GetCharacterMovement _asthird_person_character) 8.0))

(event Custom|EclateLuiSaMere
  (bind _newtrack_0 (Timeline|BoomeLe PlayFromStart)
    (:Update
      (Transformation|SetRelativeLocation (Variables|Default|GetStaticMeshDroite) (Math|Vector|Lerp(Vector) (Math|Vector|MakeVector (* (Variables|Default|GetDistance) 1.0) 0.0 0.0) (Variables|Default|GetFinish%20location%20Droite) _newtrack_0) false false)
      (Transformation|SetRelativeLocation (Variables|Default|GetStaticMeshGauche) (Math|Vector|Lerp(Vector) (Math|Vector|MakeVector (* (Variables|Default|GetDistance) -1.0) 0.0 0.0) (Variables|Default|GetFinish%20location%20Gauche) _newtrack_0) false false))
    (:Finished
      (Utilities|FlowControl|Delay 0.3)
      (bind _newtrack_0_2 (Timeline|Timeline_0 ReverseFromEnd)
        (:Update
          (Transformation|SetRelativeLocation (Variables|Default|GetStaticMeshDroite) (Math|Vector|Lerp(Vector) (Math|Vector|MakeVector (* (Variables|Default|GetDistance) 1.0) 0.0 0.0) (Variables|Default|GetFinish%20location%20Droite) _newtrack_0_2) false false)
          (Transformation|SetRelativeLocation (Variables|Default|GetStaticMeshGauche) (Math|Vector|Lerp(Vector) (Math|Vector|MakeVector (* (Variables|Default|GetDistance) -1.0) 0.0 0.0) (Variables|Default|GetFinish%20location%20Gauche) _newtrack_0_2) false false))
        (:Finished
          (Utilities|FlowControl|Delay (Utilities|Array|Get(acopy) (Variables|Default|GetDelay) (Variables|Default|GetCount)))
          (Variables|Default|SetCount (Math|Integer|SelectInt 0 (+ (Variables|Default|GetCount) 1) (> (+ (Variables|Default|GetCount) 1) (Utilities|Array|LastIndex (Variables|Default|GetDelay)))))
          (CallFunction|EclateLuiSaMere))))))

(event EventBeginPlay
  (bind _playrate (Variables|Default|GetPlayRate))
  (Variables|Default|SetFinish%20location%20Gauche (* "1.000000, 0,0.000000" (Variables|Default|GetDistance)))
  (Variables|Default|SetFinish%20location%20Droite (* "-1.000000, 0,0.000000" (Variables|Default|GetDistance)))
  (Components|Timeline|SetPlayRate (Variables|Default|GetTimeline_0) _playrate)
  (Components|Timeline|SetPlayRate (Variables|Default|GetBoomeLe) _playrate)
  (CallFunction|EclateLuiSaMere))

(event EventTick
  (params (DeltaSeconds :type Float%20%28single-precision%29))
  (if (and (Variables|Default|GetOverlapDroite) (Variables|Default|GetOverlapGauche))
    (Actor|DestroyActor (.AsThird%20Person%20Character (Utilities|Casting|CastToThirdPersonCharacter (Game|GetPlayerCharacter 0))))))

(fn ConstructionScript
  (Components|StaticMesh|SetStaticMesh (Variables|Default|GetStaticMeshGauche) (Variables|Default|GetMeshLeft))
  (Components|StaticMesh|SetStaticMesh (Variables|Default|GetStaticMeshDroite) (Variables|Default|GetMeshRight))
  (Transformation|SetRelativeLocation (Variables|Default|GetStaticMeshDroite) (Math|Vector|MakeVector (Variables|Default|GetDistance) 0.0 0.0) false false)
  (Transformation|SetRelativeLocation (Variables|Default|GetStaticMeshGauche) (Math|Vector|MakeVector (* (Variables|Default|GetDistance) -1.0) 0.0 0.0) false false))