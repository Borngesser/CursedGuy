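; Dyson fan trap that intermittently launches players upward while they are in its box volume.
; A looping timer alternates an active phase of fixed length with pauses cycled from a Delay array, toggling box visibility.
; On activation or entry while active, players get an upward impulse and lower gravity scale, raised again on exit.
; The mesh spins on Tick, and the construction script sets mesh, height and volume scale.
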(event OnComponentBeginOverlap(Box)
  (params (OverlappedComponent :type Primitive%20Component%20Object%20Reference) (OtherActor :type Actor%20Object%20Reference) (OtherComp :type Primitive%20Component%20Object%20Reference) (OtherBodyIndex :type Integer) (bFromSweep :type Boolean) (SweepResult :type Hit%20Result%20Structure%20%28by%20ref%29))
  (bind _asplayer (Utilities|Casting|CastToPlayer OtherActor))
  (if (Variables|Default|GetIsActive)
    (Physics|AddImpulse (Variables|/Script/Engine.Character|GetCharacterMovement _asplayer) (Math|Vector|MakeVector 0.0 0.0 (Variables|Default|GetPower)) true)
    (Variables|/Script/Engine.CharacterMovementComponent|SetGravityScale (Variables|/Script/Engine.Character|GetCharacterMovement _asplayer) 1.0)))

(event OnComponentEndOverlap(Box)
  (params (OverlappedComponent :type Primitive%20Component%20Object%20Reference) (OtherActor :type Actor%20Object%20Reference) (OtherComp :type Primitive%20Component%20Object%20Reference) (OtherBodyIndex :type Integer))
  (bind _asplayer (Utilities|Casting|CastToPlayer OtherActor))
  (Development|PrintString "EndOverlap")
  (Variables|/Script/Engine.CharacterMovementComponent|SetGravityScale (Variables|/Script/Engine.Character|GetCharacterMovement _asplayer) 1.8))

(event Custom|LoopVentilation
  ;[1 1 1] Temps de ventilation
  (Rendering|ToggleVisibility (Variables|Default|GetBox) false)
  (Variables|Default|SetIsActive true)
  (CallFunction|ActorInside)
  (Utilities|FlowControl|Delay (Variables|Default|GetTime))
  (Variables|Default|SetIsActive false)
  (Rendering|ToggleVisibility (Variables|Default|GetBox) false)
  ;[1 1 1] Delay
  (Utilities|FlowControl|Delay (Utilities|Array|Get(acopy) (Variables|Default|GetDelay) (Variables|Default|GetCount)))
  (Variables|Default|SetCount (Math|Integer|SelectInt 0 (+ (Variables|Default|GetCount) 1) (> (+ (Variables|Default|GetCount) 1) (Utilities|Array|LastIndex (Variables|Default|GetDelay)))))
  (CallFunction|LoopVentilation))

(event Custom|ActorInside
  (for _array_element (Collision|GetOverlappingActors (Variables|Default|GetBox) "/Game/Blueprints/Player/Player.Player_C" :!class /Script/Engine.PrimitiveComponent)
    (bind _asplayer (Utilities|Casting|CastToPlayer _array_element))
    (if (Variables|Default|GetIsActive)
      (Variables|/Script/Engine.MovementComponent|SetVelocity (Variables|/Script/Engine.Character|GetCharacterMovement _asplayer) (Math|Vector|MakeVector 0.0 0.0 (.z (Variables|/Script/Engine.MovementComponent|GetVelocity (Variables|/Script/Engine.Character|GetCharacterMovement _asplayer)))))
      (Physics|AddImpulse (Variables|/Script/Engine.Character|GetCharacterMovement _asplayer) (Math|Vector|MakeVector 0.0 0.0 (Variables|Default|GetPower)) true)
      (Variables|/Script/Engine.CharacterMovementComponent|SetGravityScale (Variables|/Script/Engine.Character|GetCharacterMovement _asplayer) 1.0))))

(event EventBeginPlay
  (CallFunction|LoopVentilation)
  (AddComponent|AddRotatingMovementComponent))

(event EventTick
  (params (DeltaSeconds :type Float%20%28single-precision%29))
  (Transformation|AddLocalRotation (Variables|Default|GetStaticMesh) "0,4.000000, 0" false false))

(fn ConstructionScript
  (bind _scene (Variables|Default|GetScene))
  (bind _returnvalue (Transformation|GetWorldTransform _scene))
  (Components|StaticMesh|SetStaticMesh (Variables|Default|GetStaticMesh) (Variables|Default|GetMesh))
  (Transformation|SetRelativeLocation (Variables|Default|GetScene) (Math|Vector|MakeVector 0.0 0.0 (Variables|Default|Getheight)) false false)
  (Transformation|SetWorldTransform _scene (Math|Transform|MakeTransform (.location _returnvalue) (.rotation _returnvalue) (Math|Vector|MakeVector 3.0 3.0 (Variables|Default|GetHauteurDeLaBox))) false false))