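; BP_Hole is a falling floor-tile trap that drops once the player steps on it.
; A player overlap on the Box fires once, waits briefly, then enables physics on the mesh and plays a 2D trap sound.
; A hit on the mesh starts a DelayDestroy countdown, after which the actor destroys itself.
; The construction script picks one of five plate meshes from the Mesh variable.
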(event OnComponentBeginOverlap(Box)
  (params (OverlappedComponent :type Primitive%20Component%20Object%20Reference) (OtherActor :type Actor%20Object%20Reference) (OtherComp :type Primitive%20Component%20Object%20Reference) (OtherBodyIndex :type Integer) (bFromSweep :type Boolean) (SweepResult :type Hit%20Result%20Structure%20%28by%20ref%29))
  ;[1 1 1] Set la physics quand le joueur marche dessus
  (Utilities|Casting|CastToPlayer OtherActor)
  (Utilities|FlowControl|DoOnce false
    (:Completed
      (Utilities|FlowControl|Delay 0.5)
      (Physics|SetSimulatePhysics (Variables|Default|GetStaticMesh) true)
      (Audio|PlaySound2D "/Game/Sound/TRAP/CUE_TRAP_Dalle.CUE_TRAP_Dalle" 1.0 1.0 0.0 0 0))))

(event OnComponentHit(StaticMesh)
  (params (HitComponent :type Primitive%20Component%20Object%20Reference) (OtherActor :type Actor%20Object%20Reference) (OtherComp :type Primitive%20Component%20Object%20Reference) (NormalImpulse :type Vector :default "0, 0, 0") (Hit :type Hit%20Result%20Structure%20%28by%20ref%29))
  ;[1 1 1] La platforme disparait au bout de "Delay" secondes
  (Utilities|FlowControl|Delay (Variables|Default|GetDelayDestroy))
  (Utilities|IsValid (Variables|Default|GetStaticMesh)
    (:Is%20Valid
      (Actor|DestroyActor))))

(fn ConstructionScript
  (Components|StaticMesh|SetStaticMesh (Variables|Default|GetStaticMesh) (Utilities|Select :Index (Variables|Default|GetMesh) :Option%200 "/Game/Mesh/Traps/PiegeDallesTombantes/PlaquesQuiTombent_Unreal_plaqueBase.PlaquesQuiTombent_Unreal_plaqueBase" :Option%201 "/Game/Mesh/Traps/PiegeDallesTombantes/PlaquesQuiTombent_Unreal_plaqueItration2.PlaquesQuiTombent_Unreal_plaqueItration2" :Option%202 "/Game/Mesh/Traps/PiegeDallesTombantes/PlaquesQuiTombent_Unreal_plaqueItération1.PlaquesQuiTombent_Unreal_plaqueItération1" :Option%203 "/Game/Mesh/Traps/PiegeDallesTombantes/PlaquesQuiTombent_Unreal_plaqueItération3.PlaquesQuiTombent_Unreal_plaqueItération3" :Option%204 "/Game/Mesh/Traps/PiegeDallesTombantes/PlaquesQuiTombent_Unreal_plaqueItération4.PlaquesQuiTombent_Unreal_plaqueItération4")))