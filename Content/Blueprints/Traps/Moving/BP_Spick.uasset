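; BP_Spick is a looping spike trap that destroys the player's ThirdPersonCharacter on overlap while active.
; The Spick timeline, scaled by PlayRate, moves the mesh vertically up to Height, then replays after waits cycled from the Delay array.
; A timeline event track flip-flops SpickActive, which gates a per-tick Box overlap check and a one-time destroy.
; The construction script assigns a cube mesh.
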(event Custom|SpickLoop
  (bind _staticmesh (Variables|Default|GetStaticMesh))
  (bind _relativelocation (Variables|/Script/Engine.SceneComponent|GetRelativeLocation _staticmesh))
  (bind _movement (Timeline|Spick PlayFromStart)
    (:Update
      (Transformation|SetRelativeLocation _staticmesh (Math|Vector|MakeVector (.x _relativelocation) (.y _relativelocation) (Math|Float|MapRangeClamped _movement 0.0 1.0 0.0 (Variables|Default|GetHeight))) false false))
    (:Finished
      (Utilities|FlowControl|Delay (Utilities|Array|Get(acopy) (Variables|Default|GetDelay) (Variables|Default|GetCount)))
      (Variables|Default|SetCount (Math|Integer|SelectInt 0 (+ (Variables|Default|GetCount) 1) (> (+ (Variables|Default|GetCount) 1) (Utilities|Array|LastIndex (Variables|Default|GetDelay)))))
      (CallFunction|SpickLoop))
    (:SetBool
      (bind _isa (Utilities|FlowControl|FlipFlop)
        (:A
          _)
        (:B
          _))
      (Variables|Default|SetSpickActive _isa))))

(event EventTick
  (params (DeltaSeconds :type Float%20%28single-precision%29))
  (bind _returnvalue (Game|GetPlayerCharacter 0))
  (bind _asthird_person_character (Utilities|Casting|CastToThirdPersonCharacter _returnvalue))
  (if (Variables|Default|GetSpickActive)
    (if (Collision|IsOverlappingActor (Variables|Default|GetBox) _asthird_person_character :!class /Script/Engine.PrimitiveComponent)
      (Utilities|FlowControl|DoOnce false
        (:Completed
          (Actor|DestroyActor _asthird_person_character))))))

(event EventBeginPlay
  (Components|Timeline|SetPlayRate (Variables|Default|GetSpick) (Variables|Default|GetPlayRate))
  (CallFunction|SpickLoop))

(fn ConstructionScript
  (Components|StaticMesh|SetStaticMesh (Variables|Default|GetStaticMesh) "/Game/Mesh/Geometry/1M_Cube.1M_Cube"))