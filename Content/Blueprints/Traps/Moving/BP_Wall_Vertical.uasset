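; Vertical crusher trap that slams a configurable mesh down a set distance and ragdolls players it catches.
; A Movement timeline drives the swept slam and arms the kill box, then a Reload timeline repositions the mesh.
; Infinite mode loops through an array of delays; otherwise a trigger box at the bottom position starts each slam.
; The kill box only kills players who are not falling while the smash is armed.
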(event OnComponentBeginOverlap(Box)
  (params (OverlappedComponent :type Primitive%20Component%20Object%20Reference) (OtherActor :type Actor%20Object%20Reference) (OtherComp :type Primitive%20Component%20Object%20Reference) (OtherBodyIndex :type Integer) (bFromSweep :type Boolean) (SweepResult :type Hit%20Result%20Structure%20%28by%20ref%29))
  (bind _asplayer (Utilities|Casting|CastToPlayer OtherActor))
  (if (and (not (AI|Components|NavMovement|IsFalling (Variables|/Script/Engine.Character|GetCharacterMovement _asplayer))) (Variables|Default|GetCanSmash))
    (Variables|/Game/Blueprints/Player/Player.Player_C|SetIsDead _asplayer true)
    (Default|Ragdoll _asplayer)))

(event OnComponentBeginOverlap(Box1)
  (params (OverlappedComponent :type Primitive%20Component%20Object%20Reference) (OtherActor :type Actor%20Object%20Reference) (OtherComp :type Primitive%20Component%20Object%20Reference) (OtherBodyIndex :type Integer) (bFromSweep :type Boolean) (SweepResult :type Hit%20Result%20Structure%20%28by%20ref%29))
  ;[1 1 1] Ecrase
  (Utilities|Casting|CastToPlayer OtherActor)
  (if (not (Variables|Default|GetIsInfinite))
    (bind _movement (Timeline|Movement PlayFromStart)
      (:Update
        (Transformation|SetRelativeLocation (Variables|Default|GetStaticMesh) (Math|Vector|Lerp(Vector) "0, 0, 0" (Variables|Default|GetFinish%20location) _movement) true false))
      (:Finished
        ;[1 1 1] Reload
        (Utilities|FlowControl|Delay 0.2)
        (Variables|Default|SetCanSmash false)
        (bind _reload (Timeline|Reload PlayFromStart)
          (:Update
            (Transformation|SetRelativeLocation (Variables|Default|GetStaticMesh) (Math|Vector|Lerp(Vector) "0, 0, 0" (Variables|Default|GetFinish%20location) _reload) false false))
          (:Finished
            (if (Variables|Default|GetIsInfinite)
              ;[1 1 1] Delay
              (Utilities|FlowControl|Delay (Utilities|Array|Get(acopy) (Variables|Default|GetDelay) (Variables|Default|GetCount)))
              (Variables|Default|SetCount (Math|Integer|SelectInt 0 (+ (Variables|Default|GetCount) 1) (> (+ (Variables|Default|GetCount) 1) (Utilities|Array|LastIndex (Variables|Default|GetDelay)))))
              (CallFunction|EcraseLeWesh)
              (else
                (CallFunction|ResetTimeline))))))
      (:SetBool
        (Variables|Default|SetCanSmash true)))))

(event Custom|EcraseLeWesh
  ;[1 1 1] Ecrase
  (bind _movement (Timeline|Movement PlayFromStart)
    (:Update
      (Transformation|SetRelativeLocation (Variables|Default|GetStaticMesh) (Math|Vector|Lerp(Vector) "0, 0, 0" (Variables|Default|GetFinish%20location) _movement) true false))
    (:Finished
      ;[1 1 1] Reload
      (Utilities|FlowControl|Delay 0.2)
      (Variables|Default|SetCanSmash false)
      (bind _reload (Timeline|Reload PlayFromStart)
        (:Update
          (Transformation|SetRelativeLocation (Variables|Default|GetStaticMesh) (Math|Vector|Lerp(Vector) "0, 0, 0" (Variables|Default|GetFinish%20location) _reload) false false))
        (:Finished
          (if (Variables|Default|GetIsInfinite)
            ;[1 1 1] Delay
            (Utilities|FlowControl|Delay (Utilities|Array|Get(acopy) (Variables|Default|GetDelay) (Variables|Default|GetCount)))
            (Variables|Default|SetCount (Math|Integer|SelectInt 0 (+ (Variables|Default|GetCount) 1) (> (+ (Variables|Default|GetCount) 1) (Utilities|Array|LastIndex (Variables|Default|GetDelay)))))
            (CallFunction|EcraseLeWesh)
            (else
              (CallFunction|ResetTimeline))))))
    (:SetBool
      (Variables|Default|SetCanSmash true))))

(event Custom|ResetTimeline
  ;[1 1 1] Ecrase
  (bind _movement (Timeline|Movement SetNewTime)
    (:Update
      (Transformation|SetRelativeLocation (Variables|Default|GetStaticMesh) (Math|Vector|Lerp(Vector) "0, 0, 0" (Variables|Default|GetFinish%20location) _movement) true false))
    (:Finished
      ;[1 1 1] Reload
      (Utilities|FlowControl|Delay 0.2)
      (Variables|Default|SetCanSmash false)
      (bind _reload (Timeline|Reload PlayFromStart)
        (:Update
          (Transformation|SetRelativeLocation (Variables|Default|GetStaticMesh) (Math|Vector|Lerp(Vector) "0, 0, 0" (Variables|Default|GetFinish%20location) _reload) false false))
        (:Finished
          (if (Variables|Default|GetIsInfinite)
            ;[1 1 1] Delay
            (Utilities|FlowControl|Delay (Utilities|Array|Get(acopy) (Variables|Default|GetDelay) (Variables|Default|GetCount)))
            (Variables|Default|SetCount (Math|Integer|SelectInt 0 (+ (Variables|Default|GetCount) 1) (> (+ (Variables|Default|GetCount) 1) (Utilities|Array|LastIndex (Variables|Default|GetDelay)))))
            (CallFunction|EcraseLeWesh)
            (else
              (CallFunction|ResetTimeline))))))
    (:SetBool
      (Variables|Default|SetCanSmash true))))

(event EventBeginPlay
  ;[1 1 1] Begin play
  (Components|Timeline|SetPlayRate (Variables|Default|GetMovement) (Variables|Default|GetPlayRate))
  (bind _output_get (Variables|Default|SetFinish%20location (* "0.000000, 0,-1.000000" (Variables|Default|GetDistance))))
  (Transformation|SetRelativeLocation (Variables|Default|GetBox1) _output_get false false)
  (if (Variables|Default|GetIsInfinite)
    (CallFunction|EcraseLeWesh)))

(fn ConstructionScript
  (Components|StaticMesh|SetStaticMesh (Variables|Default|GetStaticMesh) (Variables|Default|GetMesh)))