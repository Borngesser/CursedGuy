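; Player controller that handles the pause menu and counts elapsed play time in minutes and seconds.
; The Pause input creates or removes the HUD_Pause widget, toggling game pause and restoring viewport focus on close.
; Tick uses a one-second Delay as a timer, writing the count to Player_GI, whose values reset on BeginPlay.
; Any key press also records whether the input comes from a gamepad.
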(event EventTick
  (params (DeltaSeconds :type Float%20%28single-precision%29))
  (bind _returnvalue (Game|GetGameInstance))
  (bind _asplayer_gi (Utilities|Casting|CastToPlayer_GI _returnvalue))
  (Utilities|FlowControl|Delay 1.0)
  (if (< (Variables|Default|GetSecondes) 59)
    (bind _result (Math|Integer|IncrementInt (Variables|Default|GetSecondes))
      (:%20%20
        (Variables|/Game/Blueprints/Player/Player_GI.Player_GI_C|SetSecondesPERSO _asplayer_gi _result)))
    (else
      (bind _result_2 (Math|Integer|IncrementInt (Variables|Default|GetMinutes))
        (:%20%20
          (bind _output_get (Variables|Default|SetSecondes 0))
          (Variables|/Game/Blueprints/Player/Player_GI.Player_GI_C|SetSecondesPERSO _asplayer_gi _output_get)
          (Variables|/Game/Blueprints/Player/Player_GI.Player_GI_C|SetMinutesPERSO _asplayer_gi _result_2))))))

(event EventBeginPlay
  (bind _asplayer_gi (Utilities|Casting|CastToPlayer_GI (Game|GetGameInstance)))
  (Variables|/Game/Blueprints/Player/Player_GI.Player_GI_C|SetMinutesPERSO _asplayer_gi 0)
  (Variables|/Game/Blueprints/Player/Player_GI.Player_GI_C|SetSecondesPERSO _asplayer_gi 0))

(event Input|ActionEvents|InputActionPause
  (params (Key :type Key%20Structure :default "None"))
  (:Pressed
    (Utilities|FlowControl|FlipFlop
      (:A
        (Variables|Default|GetHUD_Pause
          (:then
            (Development|PrintString "Is Valid" :!label _label)
            (Widget|RemovefromParent (stale _hud_pause))
            (Variables|Default|SetHUD_Pause 0)
            (Game|SetGamePaused false)
            (Variables|/Script/Engine.PlayerController|SetbShowMouseCursor (Game|GetPlayerController 0) false)
            (Class|WidgetBlueprintLibrary|SetFocustoGameViewport))
          (:else
            (Development|PrintString "1ere fois")
            (bind _returnvalue (UserInterface|CreateWidget "/Game/Widgets/HUD_Pause.HUD_Pause_C" :!label _label_2))
            (bind _output_get (Variables|Default|SetHUD_Pause _returnvalue))
            (UserInterface|Viewport|AddtoViewport _output_get 0)
            (Game|SetGamePaused true))))
      (:B
        (bind _hud_pause (Variables|Default|GetHUD_Pause)
          (:then
            (goto _label))
          (:else
            (Development|PrintString "Is not valid")
            (goto _label_2)))))))

(event Input|KeyboardEvents|AnyKey
  (params (Key :type Key%20Structure :default "None"))
  (:Pressed
    (Variables|Default|SetGamepad? (Class|KismetInputLibrary|KeyIsGamepadKey Key))))

(fn ConstructionScript)